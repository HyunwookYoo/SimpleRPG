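; BP_MainPlayerController is a player controller Blueprint that adds animated transitions to showing and removing the pause menu.
; Both pause menu events run their parent implementation, then cast the inherited PauseMenu widget to WBP_PauseMenu and play its show or remove animation.
; Removal waits through a short fixed delay after starting the animation before hiding the widget, rather than listening for the animation to finish.
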(event EventDisplayPauseMenu
  (|CallParentFunction)
  (bind _aswbp_pause_menu (Utilities|Casting|CastToWBP_PauseMenu (Variables|Default|GetPauseMenu)))
  (UserInterface|Animation|PlayAnimation _aswbp_pause_menu (Variables|/Game/HUD/WBP_PauseMenu.WBP_PauseMenu_C|GetPauseMenuAnimation _aswbp_pause_menu) 0.0 1 "Forward" 1.0 false))

(event EventRemovePauseMenu
  (|CallParentFunction)
  (bind _aswbp_pause_menu (Utilities|Casting|CastToWBP_PauseMenu (Variables|Default|GetPauseMenu)))
  (UserInterface|Animation|PlayAnimation _aswbp_pause_menu (Variables|/Game/HUD/WBP_PauseMenu.WBP_PauseMenu_C|GetRemovePauseMenuAnimation _aswbp_pause_menu) 0.0 1 "Forward" 1.0 false)
  (Utilities|FlowControl|Delay 0.2)
  (Widget|SetVisibility (Variables|Default|GetPauseMenu) "Hidden"))

(fn ConstructionScript)